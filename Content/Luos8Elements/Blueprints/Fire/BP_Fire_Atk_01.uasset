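; BP_Fire_Atk_01 is a fireball attack projectile that deals damage to a Player through its health component.
; Fire launches it toward a destination by setting ProjectileMovement velocity from a suggested custom-arc trajectory.
; When its sphere begins overlapping, it queries pawns and world-static objects around the sweep location, breaks at the first successful Player cast, then applies fixed damage.
; Print strings report launch and damage for debugging.
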(event `self.Sphere.OnComponentBeginOverlap`
  (params (OverlappedComponent :type "PrimitiveComponent Object Reference") (OtherActor :type "Actor Object Reference") (OtherComp :type "PrimitiveComponent Object Reference") (OtherBodyIndex :type Integer) (bFromSweep :type Boolean) (SweepResult :type "HitResult Structure (by ref)"))
  (bind _output_get (set `self.Sweep Result` SweepResult))
  (bind _outactors (`KismetSystemLibrary.SphereOverlapActors` (`.Location` (`GameplayStatics.BreakHitResult` _output_get)) 350.0 (`|MakeArray` "ObjectTypeQuery3" "ObjectTypeQuery1" :!type "EObjectTypeQuery Enum")))
  (for _array_element _outactors
    (bind _asplayer (cast `/Game/AnimStarterPack/Player/Player` _array_element))
    (break))
  (`/Game/AI/HealthComp.SetDamage` (`/Game/AnimStarterPack/Player/Player.HealthComp` _asplayer) 5)
  (`KismetSystemLibrary.PrintString` "FieBall Setdamage"))

(fn `Fire`
  (params (Dest :type "Vector Structure"))
  (bind (_outlaunchvelocity _returnvalue) (`GameplayStatics.SuggestProjectileVelocity_CustomArc` (`self.K2_GetActorLocation`) (`KismetMathLibrary.MakeVector` Dest_X Dest_Y Dest_Z)))
  (if _returnvalue
    (bind _output_get (set `MovementComponent.Velocity` _outlaunchvelocity (`self.ProjectileMovement`)))
    (`KismetSystemLibrary.PrintString` (`KismetStringLibrary.Conv_VectorToString` _output_get))
    (else
      (`KismetSystemLibrary.PrintString` "Hello"))))

(fn `UserConstructionScript`
  (`parent.UserConstructionScript`))