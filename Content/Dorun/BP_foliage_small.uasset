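; Small foliage actor that can grow from its current scale when triggered and collapse back to zero.
; Grow sets a growing flag, and Tick then raises height and horizontal size by fixed, frame-rate-dependent steps up to separate caps, width climbing faster.
; Scale is reapplied only while height is still growing.
; DD stops growth and resets both sizes and the actor scale to zero.
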(event `self.ReceiveBeginPlay`
  (bind _size_xy (`self.size_xy`))
  (`self.SetActorScale3D` (`KismetMathLibrary.MakeVector` _size_xy _size_xy (`self.size`))))

(event `self.ReceiveTick`
  (params (DeltaSeconds :type "Float (single-precision)"))
  (bind _size (`self.size`))
  (bind _size_xy (`self.size_xy`))
  (`|ExecutionSequence`
    (:`then_0`
      (if (and (< _size 2.0) (`self.is_growing`))
        (bind _output_get (set `self.size` (+ _size 0.03)))
        (`self.SetActorScale3D` (`KismetMathLibrary.MakeVector` (stale _output_get_2) (stale _output_get_2) _output_get))))
    (:`then_1`
      (if (and (< _size_xy 3.0) (`self.is_growing`))
        (bind _output_get_2 (set `self.size_xy` (+ _size_xy 0.3)))))))

(fn `DD`
  (set `self.is_growing` false)
  (set `self.size` 0.0)
  (set `self.size_xy` 0.0)
  (`self.SetActorScale3D` (0.0 0.0 0.0)))

(fn `grow`
  (set `self.is_growing` true))

(fn `UserConstructionScript`)