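; Frost Giant enemy Blueprint that handles melee damage against the player through hitboxes on both hands.
; The construction script snaps the AttackRight and AttackLeft components to hand sockets on the mesh and collects them in an array.
; BeginAttack and EndAttack switch collision on that array on and off.
; An overlap with a Player damages its HealthComp, with a DidAttack flag limiting damage to one hit until EndAttack resets it.
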(event `self.BeginAttack`
  (for _array_element (`self.NewVar_0`)
    (`PrimitiveComponent.SetCollisionEnabled` _array_element "QueryAndPhysics")))

(event `self.EndAttack`
  (for _array_element (`self.NewVar_0`)
    (`PrimitiveComponent.SetCollisionEnabled` _array_element "NoCollision")
    (set `self.DidAttack` false)))

(event `self.AttackRight.OnComponentBeginOverlap`
  (params (OverlappedComponent :type "PrimitiveComponent Object Reference") (OtherActor :type "Actor Object Reference") (OtherComp :type "PrimitiveComponent Object Reference") (OtherBodyIndex :type Integer) (bFromSweep :type Boolean) (SweepResult :type "HitResult Structure (by ref)"))
  (bind _asplayer (cast `/Game/AnimStarterPack/Player/Player` OtherActor))
  (if (not (`self.DidAttack`))
    (set `self.DidAttack` true)
    (`/Game/AI/HealthComp.SetDamage` (`self.GetComponentByClass` _asplayer "/Game/AI/HealthComp.HealthComp_C") (`self.Damage`))))

(event `self.AttackLeft.OnComponentBeginOverlap`
  (params (OverlappedComponent :type "PrimitiveComponent Object Reference") (OtherActor :type "Actor Object Reference") (OtherComp :type "PrimitiveComponent Object Reference") (OtherBodyIndex :type Integer) (bFromSweep :type Boolean) (SweepResult :type "HitResult Structure (by ref)"))
  (bind _asplayer (cast `/Game/AnimStarterPack/Player/Player` OtherActor))
  (if (not (`self.DidAttack`))
    (set `self.DidAttack` true)
    (`/Game/AI/HealthComp.SetDamage` (`self.GetComponentByClass` _asplayer "/Game/AI/HealthComp.HealthComp_C") (`self.Damage`))))

(fn `UserConstructionScript`
  (bind _attackright (`self.AttackRight`))
  (bind _attackleft (`self.AttackLeft`))
  (bind _mesh (`self.Mesh`))
  (`KismetArrayLibrary.Array_Add` (`self.NewVar_0`) _attackright)
  (`KismetArrayLibrary.Array_Add` (`self.NewVar_0`) _attackleft)
  (`SceneComponent.K2_AttachToComponent` _attackright _mesh "RIghtHand_Socket" "SnapToTarget" "KeepRelative" "KeepRelative" true)
  (`SceneComponent.K2_AttachToComponent` _attackleft _mesh "LeftHand_Socket" "SnapToTarget" "KeepRelative" "KeepRelative" true))