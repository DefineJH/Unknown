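; Anim notify state, shown as AttackBreath, that switches the boss AI character's breath attack on for a window of an animation.
; On begin it casts the mesh owner to AICharacter_Boss_BP and calls SetBreath, and on end it calls DisableBreath.
; Tick does no work, and owners that are not that boss class are ignored.
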(fn `GetNotifyName`
  (returns (ReturnValue :type String))
  (return "AttackBreath"))

(fn `Received_NotifyBegin`
  (params (MeshComp :type "SkeletalMeshComponent Object Reference") (Animation :type "AnimSequenceBase Object Reference") (TotalDuration :type "Float (double-precision)"))
  (returns (ReturnValue :type Boolean))
  (bind _asaicharacter_boss_bp (cast `/Game/AI/Boss/AICharacter_Boss_BP` (`ActorComponent.GetOwner` MeshComp)))
  (`/Game/AI/Boss/AICharacter_Boss_BP.SetBreath` _asaicharacter_boss_bp)
  (bind _returnvalue (`parent.Received_NotifyBegin` MeshComp Animation TotalDuration))
  (return _returnvalue))

(fn `Received_NotifyEnd`
  (params (MeshComp :type "SkeletalMeshComponent Object Reference") (Animation :type "AnimSequenceBase Object Reference"))
  (returns (ReturnValue :type Boolean))
  (bind _asaicharacter_boss_bp (cast `/Game/AI/Boss/AICharacter_Boss_BP` (`ActorComponent.GetOwner` MeshComp)))
  (`/Game/AI/Boss/AICharacter_Boss_BP.DisableBreath` _asaicharacter_boss_bp)
  (bind _returnvalue (`parent.Received_NotifyEnd` MeshComp Animation))
  (return _returnvalue))

(fn `Received_NotifyTick`
  (params (MeshComp :type "SkeletalMeshComponent Object Reference") (Animation :type "AnimSequenceBase Object Reference") (FrameDeltaTime :type "Float (double-precision)"))
  (returns (ReturnValue :type Boolean))
  (return false))